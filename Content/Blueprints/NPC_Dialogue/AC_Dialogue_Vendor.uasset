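; Vendor NPC dialogue component that runs a branching conversation offering to buy the player's scrap.
; It overrides the parent Dialogue graph, switching on a tree index and chaining AddDialogue nodes whose option results drive the branches.
; Declining sets the index so later talks open with a random grumpy greeting before looping back to the offer.
; Accepting only prints a placeholder string.
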(fn `Dialogue`
  (`parent.Dialogue`)
  (switch `int` (`self.DialogueTreeIndex`)
    (:`0`
      _)
    (:`1`
      ;[1 1 1] Remembers the player
      (bind _state (`self.AddDialogue` "Vendor" (select `int` (`KismetMathLibrary.RandomIntegerInRange` 0 2) :`0` "Here to waste my time again?" :`1` "Oh..its you again" :`2` "Welcome..oh its you" :!type "Text") (`|MakeArray` "Im back!" :!type "Text")))
      (switch `/Game/Blueprints/NPC_Dialogue/Enum_Dialogue` _state
        (:`NewEnumerator0`
          (switch `int` 0
            (:`0`
              _))))))
  (bind (_state_2 _optioninteger) (`self.AddDialogue` "Vendor" "Are you looking to sell your scrap?" (`|MakeArray` "Yes" "No" :!type "Text")))
  (switch `/Game/Blueprints/NPC_Dialogue/Enum_Dialogue` _state_2
    (:`NewEnumerator0`
      (switch `int` _optioninteger
        (:`0`
          (`KismetSystemLibrary.PrintString` "Sell Scrap"))
        (:`1`
          ;[1 1 1] No, Thanks
          (bind _state_3 (`self.AddDialogue` "Vendor" "Then leave!" (`|MakeArray` "Continue" :!type "Text")))
          (switch `/Game/Blueprints/NPC_Dialogue/Enum_Dialogue` _state_3
            (:`NewEnumerator0`
              (`self.SetDialogueTreeIndex` 1)
              (`self.CloseConversation`))))))))