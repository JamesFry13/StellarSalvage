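; BP_NPC_Base is a base NPC Blueprint for dialogue, with an interaction outline and a zero hold time for interacting.
; The construction script writes the character name into a TextRender component.
; SetOutlineState toggles custom depth on the mesh for highlighting, but hides the name text in both states.
; ConversationClosed notifies the interaction instigator that the conversation has ended.
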(event `/Game/Blueprints/InteractSystem/BPI_Interact.SetOutlineState`
  (params (`bShow?` :type Boolean))
  (if `bShow?`
    (`SceneComponent.SetVisibility` (`self.TextRender`) false false)
    (`PrimitiveComponent.SetRenderCustomDepth` (`self.Mesh`) true)
    (else
      (`SceneComponent.SetVisibility` (`self.TextRender`) false false)
      (`PrimitiveComponent.SetRenderCustomDepth` (`self.Mesh`) false))))

(event `/Game/Blueprints/NPC_Dialogue/BPI_Conversation.ConversationClosed`
  (message `/Game/Blueprints/NPC_Dialogue/BPI_Conversation.ConversationClosed` (`self.InteractInstigator`)))

(fn `GetInteractHoldTime`
  (returns (HoldTime :type "Float (double-precision)"))
  (return 0.0))

(fn `UserConstructionScript`
  (`TextRenderComponent.K2_SetText` (`self.TextRender`) (`self.T_CharacterName`)))