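; Dialogue component for the Traveller NPC, holding the start of a conversation that opens with a question about cheese.
; It overrides Dialogue, calls the parent, then switches on DialogueTreeIndex, where the only branch adds the Traveller's line with two reply options.
; The switch on the chosen option is still empty, and the progress, close and tree-index calls are unwired reference nodes.
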(fn `Dialogue`
  (`parent.Dialogue`)
  (switch `int` (`self.DialogueTreeIndex`)
    (:`0`
      (bind (_state _optioninteger) (`self.AddDialogue` "Traveller" "Hi, do you have any cheese?" (`|MakeArray` "Im looking for some salvage" "No, thanks" :!type "Text")))
      (switch `/Game/Blueprints/Dialogue/Enum_Dialogue` _state
        (:`NewEnumerator0`
          (switch `int` _optioninteger))))))