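; BP_NPC_Base is the base Blueprint for dialogue NPCs that a player can interact with.
; The construction script writes the character name into a TextRender component.
; SetInteractableState hides that text whether or not interaction is available, as both branches set visibility to false.
; When a conversation closes, ConversationClosed passes the notice to InteractInstigator through ConversationClosedMessage.
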(event `/Game/Blueprints/Dialogue/BPI_Interactable.SetInteractableState`
  (params (`CanShowInteract?` :type Boolean))
  (if `CanShowInteract?`
    (`SceneComponent.SetVisibility` (`self.TextRender`) false false)
    (else
      (`SceneComponent.SetVisibility` (`self.TextRender`) false false))))

(event `/Game/Blueprints/Dialogue/BPI_Interactable.ConversationClosed`
  (message `/Game/Blueprints/Dialogue/BPI_Interactable.ConversationClosed` (`self.InteractInstigator`)))

(fn `UserConstructionScript`
  (`TextRenderComponent.K2_SetText` (`self.TextRender`) (`self.T_CharacterName`)))