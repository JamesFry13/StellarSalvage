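; Base NPC Blueprint for roaming, talkable characters that notice the player and can be highlighted for interaction.
; Pawn sensing focuses the AI controller on the player and sets the "IsNearby?" blackboard key, clearing it after a wait if no conversation started or shortly after one closes.
; A sphere overlap drives the anim instance's near-player flag and clears focus on exit.
; The interaction outline uses custom depth, and the construction script writes the character name to a text render.
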(event `/Game/Blueprints/InteractSystem/BPI_Interact.SetOutlineState`
  (params (`bShow?` :type Boolean))
  (if `bShow?`
    (`SceneComponent.SetVisibility` (`self.TextRender`) false false)
    (`PrimitiveComponent.SetRenderCustomDepth` (`self.Mesh`) true)
    (else
      (`SceneComponent.SetVisibility` (`self.TextRender`) false false)
      (`PrimitiveComponent.SetRenderCustomDepth` (`self.Mesh`) false))))

(event `/Game/Blueprints/NPCs/BPI_Conversation.ConversationClosed`
  (message `/Game/Blueprints/NPCs/BPI_Conversation.ConversationClosed` (`self.InteractInstigator`))
  ;[1 1 1] Walk off When Conversation Ended
  (`KismetSystemLibrary.Delay` 1.0)
  (`BlackboardComponent.SetValueAsBool` (`AIBlueprintHelperLibrary.GetBlackboard` (`AIBlueprintHelperLibrary.GetAIController` self)) "IsNearby?" false))

(event `self.PawnSensing.OnSeePawn`
  (params (Pawn :type "Pawn Object Reference"))
  ;[0.324 1 0.6204] NPC Stops
  (`self.LookAt`)
  (cast `/Game/Blueprints/PlayerCharacter/BP_PlayerCharacter` Pawn)
  (`BlackboardComponent.SetValueAsBool` (`AIBlueprintHelperLibrary.GetBlackboard` (`AIBlueprintHelperLibrary.GetAIController` self)) "IsNearby?" true)
  (`KismetSystemLibrary.Delay` (`self.WaitTime`))
  (if (not (`self.HasTalkedtoNPC?`))
    (`BlackboardComponent.SetValueAsBool` (`AIBlueprintHelperLibrary.GetBlackboard` (`AIBlueprintHelperLibrary.GetAIController` self)) "IsNearby?" false)))

(event `/Game/Blueprints/NPCs/BPI_Conversation.ConversationOpened`
  ;[1 1 1] Comment
  (set `self.HasTalkedtoNPC?` true))

(event `self.Sphere.OnComponentBeginOverlap`
  (params (OverlappedComponent :type "PrimitiveComponent Object Reference") (OtherActor :type "Actor Object Reference") (OtherComp :type "PrimitiveComponent Object Reference") (OtherBodyIndex :type Integer) (bFromSweep :type Boolean) (SweepResult :type "HitResult Structure (by ref)"))
  (bind _asabp_ai (cast `/Game/Blueprints/NPCs/Animations/ABP_AI` (`SkeletalMeshComponent.GetAnimInstance` (`self.Mesh`))))
  (set `/Game/Blueprints/NPCs/Animations/ABP_AI.IsNearPlayer` true _asabp_ai))

(event `self.Sphere.OnComponentEndOverlap`
  (params (OverlappedComponent :type "PrimitiveComponent Object Reference") (OtherActor :type "Actor Object Reference") (OtherComp :type "PrimitiveComponent Object Reference") (OtherBodyIndex :type Integer))
  (bind _asabp_ai (cast `/Game/Blueprints/NPCs/Animations/ABP_AI` (`SkeletalMeshComponent.GetAnimInstance` (`self.Mesh`))))
  (set `/Game/Blueprints/NPCs/Animations/ABP_AI.IsNearPlayer` false _asabp_ai)
  (`self.EndTurnAndFace`))

(fn `Begin Turn and Face`
  (`AIController.K2_SetFocus` (`AIBlueprintHelperLibrary.GetAIController` self) (`GameplayStatics.GetPlayerCharacter` 0)))

(fn `EndTurnAndFace`
  (`AIController.K2_ClearFocus` (`AIBlueprintHelperLibrary.GetAIController` self)))

(fn `GetInteractHoldTime`
  (returns (HoldTime :type "Float (double-precision)"))
  (return 0.0))

(fn `LookAt`
  (bind _asabp_ai (cast `/Game/Blueprints/NPCs/Animations/ABP_AI` (`SkeletalMeshComponent.GetAnimInstance` (`self.Mesh`))))
  (set `/Game/Blueprints/NPCs/Animations/ABP_AI.IsNearPlayer` true _asabp_ai)
  (`self.Begin Turn and Face`))

(fn `UserConstructionScript`
  (set `self.IsAbleToRoam?` (`self.IsAbleToRoam?`))
  (`TextRenderComponent.K2_SetText` (`self.TextRender`) (`self.T_CharacterName`)))