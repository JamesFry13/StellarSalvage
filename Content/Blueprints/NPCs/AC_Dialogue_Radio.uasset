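; Dialogue component for a radio conversation in which NovaCore briefs the player on recovering a crashed satellite.
; Overrides Dialogue, switching on DialogueTreeIndex (only tree 0 exists) into nested AddDialogue calls that branch on the chosen option.
; Branches loop back or converge on the briefing, with a randomized retort when the player first stays silent.
; The mission start is currently only a "Begin Mission" print.
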(fn `Dialogue`
  (`parent.Dialogue`)
  (switch `int` (`self.DialogueTreeIndex`)
    (:`0`
      ;[0.1912 1 0.4072] Comment
      (bind (_state _optioninteger) (`self.AddDialogue` "*Radio Transmission* NovaCore" "Come in...Do you read, over?" (`|MakeArray` "Uhh...who is this?" "I read you loud and clear!" "(Stay Silent)" :!type "Text") :!label _label))
      (switch `/Game/Blueprints/NPCs/Enum_Dialogue` _state
        (:`NewEnumerator0`
          (switch `int` _optioninteger
            (:`0`
              ;[0.1354 1 1] Comment
              (bind (_state_2 _optioninteger_2) (`self.AddDialogue` "*Radio Transmission* NovaCore" "...You're employer? Don't act stupid with me or i'll have you fired faster than you can say..." (`|MakeArray` "Im sorry, it was a bad joke" "...NovaCore?" :!type "Text") :!label _label_2))
              (switch `/Game/Blueprints/NPCs/Enum_Dialogue` _state_2
                (:`NewEnumerator0`
                  (switch `int` _optioninteger_2
                    (:`0`
                      ;[0.1912 1 0.4072] Comment
                      (bind (_state_3 _optioninteger_3) (`self.AddDialogue` "*Radio Transmission* NovaCore" "We just got word on a crashed satellite, naturally it will need to be recovered swiftly to avoid outlaws from obtaining it." (`|MakeArray` "I'm on it! Whats the location?" "Hold on, how much am I getting paid!" "(Keep Remaining Silent)" :!type "Text") :!label _label_3))
                      (switch `/Game/Blueprints/NPCs/Enum_Dialogue` _state_3
                        (:`NewEnumerator0`
                          (switch `int` _optioninteger_3
                            (:`0`
                              _)
                            (:`1`
                              ;[1 1 1] Comment
                              (bind (_state_4 _optioninteger_4) (`self.AddDialogue` "*Radio Transmission* NovaCore" "Check your contract, I am not obligated to share this with you!" (`|MakeArray` "Alright, fine." :!type "Text")))
                              (switch `/Game/Blueprints/NPCs/Enum_Dialogue` _state_4
                                (:`NewEnumerator0`
                                  (switch `int` _optioninteger_4
                                    (:`0`
                                      _)))))
                            (:`2`
                              ;[1 1 1] Comment
                              (bind (_state_5 _optioninteger_5) (`self.AddDialogue` "*Radio Transmission* NovaCore" "...Hello? Are you there?" (`|MakeArray` "Im here!" "No...?" :!type "Text")))
                              (switch `/Game/Blueprints/NPCs/Enum_Dialogue` _state_5
                                (:`NewEnumerator0`
                                  (switch `int` _optioninteger_5
                                    (:`0`
                                      (goto _label_3))
                                    (:`1`
                                      (bind (_state_6 _optioninteger_6) (`self.AddDialogue` "*Radio Transmission* NovaCore" "**Deep Sigh*** Where do we get these people from..." (`|MakeArray` "(Continue)" :!type "Text") :!label _label_4))
                                      (switch `/Game/Blueprints/NPCs/Enum_Dialogue` _state_6
                                        (:`NewEnumerator0`
                                          (switch `int` _optioninteger_6
                                            (:`0`
                                              (goto _label_3))))))))))))))
                    (:`1`
                      (goto _label_4))))))
            (:`1`
              (goto _label_3))
            (:`2`
              ;[0.5865 1 0.6617] Comment
              (bind (_state_7 _optioninteger_7) (`self.AddDialogue` "*Radio Transmission* NovaCore" (select `int` (`KismetMathLibrary.RandomIntegerInRange` 0 2) :`0` "...Hello! DO YOU COPY?" :`1` "Stop messing around or I'll give this contract to another employee!" :`2` "I know yopu're there, stop playing games!" :!type "Text") (`|MakeArray` "I read you loud and clear!" "Uhh...who is this?" "(Keep Remaining Silent)" :!type "Text")))
              (switch `/Game/Blueprints/NPCs/Enum_Dialogue` _state_7
                (:`NewEnumerator0`
                  (switch `int` _optioninteger_7
                    (:`0`
                      (goto _label_3))
                    (:`1`
                      (goto _label_2))
                    (:`2`
                      (goto _label)))))))
          ;[1 1 1] Begin Mission
          (bind (_state_8 _optioninteger_8) (`self.AddDialogue` "*Radio Transmission* NovaCore" "Ill go ahead and send you the coordinates now" (`|MakeArray` "What can you tell me about the place i'm going to?" "Copy, ready to receive! (Continue)" :!type "Text")))
          (switch `/Game/Blueprints/NPCs/Enum_Dialogue` _state_8
            (:`NewEnumerator0`
              (switch `int` _optioninteger_8
                (:`0`
                  (bind (_state_9 _optioninteger_9) (`self.AddDialogue` "*Radio Transmission* NovaCore" "Nothing too crazy, initial scans seem to indicate its fairly safe...just watch your step, the terrain is quite rocky." (`|MakeArray` "Thanks! (Continue)" "Anything else?" :!type "Text")))
                  (switch `/Game/Blueprints/NPCs/Enum_Dialogue` _state_9
                    (:`NewEnumerator0`
                      (switch `int` _optioninteger_9
                        (:`0`
                          _)
                        (:`1`
                          (`self.AddDialogue` "*Radio Transmission* NovaCore" "...No" (`|MakeArray` "Alright (Continue)" :!type "Text")))))))
                (:`1`
                  _))
              (`KismetSystemLibrary.PrintString` "Begin Mission"))))))))