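; Dialogue component for the Traveller NPC, who asks the player for cheese through a branching conversation.
; It overrides the parent Dialogue function, switching on DialogueTreeIndex and chaining AddDialogue calls whose chosen option picks the next line.
; Giving cheese advances to index 1, where later talks show a random happy line.
; Refusing rolls back dialogue progress, while having none clears it, before the conversation closes.
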(fn `Dialogue`
  (`parent.Dialogue`)
  (switch `int` (`self.DialogueTreeIndex`)
    (:`0`
      (bind (_state _optioninteger) (`self.AddDialogue` "Traveller" "Hi, do you have any cheese?" (`|MakeArray` "Yes" "No" :!type "Text")))
      (switch `/Game/Blueprints/NPCs/Enum_Dialogue` _state
        (:`NewEnumerator0`
          (switch `int` _optioninteger
            (:`0`
              (bind (_state_2 _optioninteger_2) (`self.AddDialogue` "Traveller" "Thats great news can I have some?" (`|MakeArray` "Give Cheese" "Keep Cheese" :!type "Text")))
              (switch `/Game/Blueprints/NPCs/Enum_Dialogue` _state_2
                (:`NewEnumerator0`
                  (switch `int` _optioninteger_2
                    (:`0`
                      (bind _state_3 (`self.AddDialogue` "Traveller" "Thank you!" (`|MakeArray` "Continue" :!type "Text")))
                      (switch `/Game/Blueprints/NPCs/Enum_Dialogue` _state_3
                        (:`NewEnumerator0`
                          (`self.SetDialogueTreeIndex` 1)
                          (`self.CloseConversation`))))
                    (:`1`
                      (bind _state_4 (`self.AddDialogue` "Traveller" "You big meanie!" (`|MakeArray` "Continue" :!type "Text")))
                      (switch `/Game/Blueprints/NPCs/Enum_Dialogue` _state_4
                        (:`NewEnumerator0`
                          (`self.RemoveDialogueProgress` 2)
                          (`self.CloseConversation`))))))))
            (:`1`
              (bind (_state_5 _optioninteger_3) (`self.AddDialogue` "Traveller" "Aww thats a shame I really want some cheese" (`|MakeArray` "Continue" :!type "Text")))
              (switch `/Game/Blueprints/NPCs/Enum_Dialogue` _state_5
                (:`NewEnumerator0`
                  (switch `int` _optioninteger_3
                    (:`0`
                      (`self.ClearDialogueProgress`)
                      (`self.CloseConversation`))))))))))
    (:`1`
      (bind _state_6 (`self.AddDialogue` "Traveller" (select `int` (`KismetMathLibrary.RandomIntegerInRange` 0 2) :`0` "Nom nom nom!" :`1` "You're the best!" :`2` "Wooo!" :!type "Text") (`|MakeArray` "Continue" :!type "Text")))
      (switch `/Game/Blueprints/NPCs/Enum_Dialogue` _state_6
        (:`NewEnumerator0`
          (`self.SetDialogueTreeIndex` 1)
          (`self.CloseConversation`))))))