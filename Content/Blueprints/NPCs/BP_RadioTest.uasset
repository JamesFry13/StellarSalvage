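; BP_RadioTest is an interactable NPC, apparently for testing radio dialogue, that opens its ACDialogueRadio conversation one second after play begins.
; Sphere overlaps and pawn sensing set IsNearPlayer on the ABP_AI animation instance, while outline toggling drives mesh custom depth and keeps the name text hidden.
; Opening a conversation records that the NPC was talked to; closing it notifies the instigator, then clears the blackboard's nearby flag so the NPC walks off.
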(event `self.ReceiveBeginPlay`
  (`KismetSystemLibrary.Delay` 1.0)
  (`/Game/Blueprints/NPCs/AC_Dialogue_Base.OpenConversation` (`self.AC_Dialogue_Radio`)))

(event `self.SetOutlineState`
  (params (`bShow?` :type Boolean))
  (if `bShow?`
    (`SceneComponent.SetVisibility` (`self.TextRender`) false false)
    (`PrimitiveComponent.SetRenderCustomDepth` (`self.Mesh`) true)
    (else
      (`SceneComponent.SetVisibility` (`self.TextRender`) false false)
      (`PrimitiveComponent.SetRenderCustomDepth` (`self.Mesh`) false))))

(event `self.ConversationClosed`
  (message `/Game/Blueprints/NPCs/BPI_Conversation.ConversationClosed` (`self.InteractInstigator`))
  ;[1 1 1] Walk off When Conversation Ended
  (`KismetSystemLibrary.Delay` 1.0)
  (`BlackboardComponent.SetValueAsBool` (`AIBlueprintHelperLibrary.GetBlackboard` (`AIBlueprintHelperLibrary.GetAIController` self)) "IsNearby?" false))

(event `self.PawnSensing.OnSeePawn`
  (params (Pawn :type "Pawn Object Reference"))
  ;[0.324 1 0.6204] NPC Stops
  (`self.TurnAndFace`))

(event `self.ConversationOpened`
  ;[1 1 1] Comment
  (set `self.HasTalkedtoNPC?` true))

(event `self.Sphere.OnComponentBeginOverlap`
  (params (OverlappedComponent :type "PrimitiveComponent Object Reference") (OtherActor :type "Actor Object Reference") (OtherComp :type "PrimitiveComponent Object Reference") (OtherBodyIndex :type Integer) (bFromSweep :type Boolean) (SweepResult :type "HitResult Structure (by ref)"))
  (bind _asabp_ai (cast `/Game/Blueprints/NPCs/Animations/ABP_AI` (`SkeletalMeshComponent.GetAnimInstance` (`self.Mesh`))))
  (set `/Game/Blueprints/NPCs/Animations/ABP_AI.IsNearPlayer` true _asabp_ai))

(event `self.Sphere.OnComponentEndOverlap`
  (params (OverlappedComponent :type "PrimitiveComponent Object Reference") (OtherActor :type "Actor Object Reference") (OtherComp :type "PrimitiveComponent Object Reference") (OtherBodyIndex :type Integer))
  (bind _asabp_ai (cast `/Game/Blueprints/NPCs/Animations/ABP_AI` (`SkeletalMeshComponent.GetAnimInstance` (`self.Mesh`))))
  (set `/Game/Blueprints/NPCs/Animations/ABP_AI.IsNearPlayer` false _asabp_ai))

(fn `GetInteractHoldTime`
  (returns (HoldTime :type "Float (double-precision)"))
  (return 0.0))

(fn `TurnAndFace`
  (bind _asabp_ai (cast `/Game/Blueprints/NPCs/Animations/ABP_AI` (`SkeletalMeshComponent.GetAnimInstance` (`self.Mesh`))))
  (set `/Game/Blueprints/NPCs/Animations/ABP_AI.IsNearPlayer` true _asabp_ai))

(fn `UserConstructionScript`
  (set `self.IsAbleToRoam?` (`self.IsAbleToRoam?`))
  (`TextRenderComponent.K2_SetText` (`self.TextRender`) (`self.T_CharacterName`)))