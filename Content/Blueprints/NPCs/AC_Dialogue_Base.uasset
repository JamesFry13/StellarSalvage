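; Base NPC dialogue component that opens and closes a WBP_Dialogue widget, switches to UI-only input and messages its owner.
; Dialogue is a stub, apparently for child trees to override with AddDialogue calls, which return saved choices or display the first unanswered line.
; Each selection is stored by index in DialogueProgress, then Dialogue reruns from the start to replay the branch.
; Helpers clear or remove progress, or switch tree index.
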(fn `AddDialogue`
  (params (Speaker :type Text) (Dialogue :type Text) (OptionsText :type "Array of Text") (CharImage :type "Texture2D Object Reference"))
  (returns (State :type "/Game/Blueprints/NPCs/Enum_Dialogue Enum") (OptionInteger :type Integer))
  (bind (_value _returnvalue) (`BlueprintMapLibrary.Map_Find` (`self.DialogueProgress`) (`self.DialogueIndex`)))
  (`/Engine/EditorBlueprintResources/StandardMacros.IncrementInt` (`self.DialogueIndex`)
    (:`  `
      (if _returnvalue
        (return "NewEnumerator0" _value)
        (else
          (`/Game/Widgets/Dialogue/WBP_Dialogue.UpdateDialogueText` (`self.DialogueWIDREF`) (`self.DialogueIndex`) (`local.Speaker`) (`local.Dialogue`) (`local.OptionsText`) (`local.CharImage`))
          (return "NewEnumerator1" 0))))))

(fn `ClearDialogueProgress`
  (`BlueprintMapLibrary.Map_Clear` (`self.DialogueProgress`)))

(fn `CloseConversation`
  (`Widget.RemoveFromParent` (`self.DialogueWIDREF`))
  (message `/Game/Blueprints/NPCs/BPI_Conversation.ConversationClosed` (`self.GetOwner`)))

(fn `Dialogue`
  (`GameplayStatics.PlaySound2D` (`self.UIPopupSound`) 1.0 1.0 0.0 null null))

(fn `OpenConversation`
  (message `/Game/Blueprints/NPCs/BPI_Conversation.ConversationOpened` (`self.GetOwner`))
  (`GameplayStatics.PlaySound2D` (`self.UIPopupSound`) 1.0 1.0 0.0 null null)
  (`WidgetBlueprintLibrary.SetInputMode_UIOnlyEx` (`GameplayStatics.GetPlayerController` 0) null)
  (set `PlayerController.bShowMouseCursor` true (`GameplayStatics.GetPlayerController` 0))
  (bind _returnvalue (`|CreateWidget` "/Game/Widgets/Dialogue/WBP_Dialogue.WBP_Dialogue_C" null self null))
  (bind _output_get (set `self.DialogueWIDREF` _returnvalue))
  (`UserWidget.AddToViewport` _output_get 0)
  (`self.ProgressDialogue`))

(fn `ProgressDialogue`
  (set `self.DialogueIndex` -1)
  (`self.Dialogue`))

(fn `RemoveDialogueProgress`
  (params (ProgressSteps :type Integer))
  (for _index (range (+ ProgressSteps 1))
    (`BlueprintMapLibrary.Map_Remove` (`self.DialogueProgress`) (- _index (`self.DialogueIndex`)))))

(fn `SetDialogueTreeIndex`
  (params (DialogueTreeIndex :type Integer))
  (set `self.DialogueTreeIndex` DialogueTreeIndex)
  (`self.ClearDialogueProgress`))

(fn `UpdateSelectedOption`
  (params (ProgressIndex :type "Integer (by ref)") (OptionIndex :type "Integer (by ref)"))
  (`BlueprintMapLibrary.Map_Add` (`self.DialogueProgress`) ProgressIndex OptionIndex)
  (`self.ProgressDialogue`))