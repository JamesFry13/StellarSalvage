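; AC_InteractionPlayer is a player interaction component that toggles outline highlights on interactable actors.
; UpdateInteractState takes a hit flag and, when true, switches on the outline of CurrentHitActor.
; In both hit and miss cases it switches off the outline of PrevHitActor if that actor is valid.
; Outline changes go through SetOutlineStateMessage calls on the target actors.
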(fn `UpdateInteractState`
  (params (`bHit?` :type Boolean))
  (if `bHit?`
    (message `/Game/Blueprints/InteractSystem/BPI_Interact.SetOutlineState` (`self.CurrentHitActor`) true)
    (`/Engine/EditorBlueprintResources/StandardMacros.IsValid` (`self.PrevHitActor`)
      (:`Is Valid`
        (message `/Game/Blueprints/InteractSystem/BPI_Interact.SetOutlineState` (`self.PrevHitActor`) false)))
    (else
      (`/Engine/EditorBlueprintResources/StandardMacros.IsValid` (`self.PrevHitActor`)
        (:`Is Valid`
          (message `/Game/Blueprints/InteractSystem/BPI_Interact.SetOutlineState` (`self.PrevHitActor`) false))))))