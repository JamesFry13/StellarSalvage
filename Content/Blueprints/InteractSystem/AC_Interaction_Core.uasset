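; AC_Interaction_Core is an interaction component that detects the actor ahead of the player and triggers interactions on it.
; A debug-drawn line trace from player 0's capsule runs on Tick or a looping timer, tracking current and previous hits.
; Target changes reset hold progress and call an empty UpdateInteractState hook.
; UpdateInteract compares supplied hold duration to the target's required time, then sends InteractMessage, using a next-tick lockout against double triggering.
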(event `self.ReceiveBeginPlay`
  (if (`self.bUpdateOnTick?`)
    (`self.SetComponentTickEnabled` true)
    (else
      (`KismetSystemLibrary.K2_SetTimer` null "TraceForInteract" (`self.UpdateFrequency`) true))))

(event `self.ReceiveTick`
  (params (DeltaSeconds :type "Float (single-precision)"))
  (`self.TraceForInteract`))

(fn `GetTraceLocations`
  (returns (Start :type "Vector Structure") (End :type "Vector Structure"))
  (bind _capsulecomponent (`Character.CapsuleComponent` (`GameplayStatics.GetPlayerCharacter` 0)))
  (bind _returnvalue (`SceneComponent.K2_GetComponentLocation` _capsulecomponent))
  (return _returnvalue (+ _returnvalue (* (`SceneComponent.GetForwardVector` _capsulecomponent) (`self.InteractDistance`)))))

(fn `RetriggerDelay`
  (if (`self.bTriggerDelay`)
    (set `self.bTriggerDelay` false)
    (else
      (set `self.bTriggerDelay` true)
      (`KismetSystemLibrary.K2_SetTimerForNextTick` null "RetriggerDelay"))))

(fn `TraceForInteract`
  (bind (_start _end) (`self.GetTraceLocations`))
  (bind (_outhit _returnvalue) (`KismetSystemLibrary.LineTraceSingle` :`Start` _start :`End` _end :`TraceChannel` "TraceTypeQuery3" :`DrawDebugType` "ForDuration"))
  (if _returnvalue
    (bind (_bblockinghit _binitialoverlap _time _distance _location _impactpoint _normal _impactnormal _physmat _hitactor) (`GameplayStatics.BreakHitResult` _outhit))
    (if (!= _hitactor (`self.CurrentHitActor`))
      (set `self.PrevHitActor` (`self.CurrentHitActor`))
      (set `self.CurrentHitActor` _hitactor)
      (set `self.bCanSetPrevious?` true)
      (set `self.CurrentHoldDuration` 0.0)
      (`self.UpdateInteractState` true :!label _label)
      (`KismetSystemLibrary.PrintString` "Interactable Found!" true true (struct :`R` 0.070054 :`G` 1.0 :`B` 0.358848 :`A` 1.0))
      (elif (`self.GetRecheckHit`)
        (`self.DisableHitRecheck`)
        (goto _label)))
    (elif (`self.bCanSetPrevious?`)
      (`self.DisableHitRecheck`)
      (`/Engine/EditorBlueprintResources/StandardMacros.IsValid` (`self.CurrentHitActor`)
        (:`Is Valid`
          (set `self.PrevHitActor` (`self.CurrentHitActor`)))
        (:`Is Not Valid`
          (set `self.PrevHitActor` null)))
      (set `self.CurrentHitActor` null)
      (set `self.bCanSetPrevious?` false)
      (set `self.CurrentHoldDuration` 0.0)
      (`self.UpdateInteractState` false)
      (`KismetSystemLibrary.PrintString` "No Interactable Found" true true (struct :`R` 1.0 :`G` 0.26725 :`B` 0.104167 :`A` 1.0)))))

(fn `TriggerInteract`
  (`self.RetriggerDelay`)
  (if (`self.GetCurrentHit`)
    (message `/Game/Blueprints/InteractSystem/BPI_Interact.Interact` (`self.CurrentHitActor`) (`self.GetOwner`))
    (set `self.CurrentHoldDuration` 0.0)))

(fn `UpdateInteract`
  (params (CurrentHoldDuration :type "Float (double-precision)"))
  (set `self.CurrentHoldDuration` CurrentHoldDuration)
  (if (`self.bTriggerDelay`)
    _
    (elif (`self.GetCurrentHit`)
      (bind _holdtime (message `/Game/Blueprints/InteractSystem/BPI_Interact.GetInteractHoldTime` (`self.CurrentHitActor`)))
      (set `self.InteractHoldTimer` _holdtime)
      (if (>= (`local.CurrentHoldDuration`) (`self.InteractHoldTimer`))
        (`self.TriggerInteract`)))))

(fn `UpdateInteractState`
  (params (`bHit?` :type Boolean)))