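; AC_InteractionBase is the base component of the interaction system, holding the shared hit state for interaction logic.
; It exposes getters for the current and previous hit actors, each paired with a validity flag.
; A RecheckHit flag can be read, enabled or disabled through simple functions.
; The graphs shown only read and toggle this state, with no detection or interaction logic.
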(fn `DisableHitRecheck`
  (set `self.bRecheckHit?` false))

(fn `EnableHitRecheck`
  (set `self.bRecheckHit?` true))

(fn `GetCurrentHit`
  (returns (ReturnValue :type Boolean) (CurrentHitActor :type "Actor Object Reference"))
  (bind _currenthitactor (`self.CurrentHitActor`))
  (return (`KismetSystemLibrary.IsValid` _currenthitactor) _currenthitactor))

(fn `GetPrevHit`
  (returns (ReturnValue :type Boolean) (PrevHitActor :type "Actor Object Reference"))
  (bind _prevhitactor (`self.PrevHitActor`))
  (return (`KismetSystemLibrary.IsValid` _prevhitactor) _prevhitactor))

(fn `GetRecheckHit`
  (returns (`bRecheckHit?` :type Boolean))
  (return (`self.bRecheckHit?`)))