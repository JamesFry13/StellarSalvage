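; BP_Salvage is an interactable salvage pile that grants the player a randomly sized amount of salvage, then destroys itself.
; Interact runs once with no hold time, calling BeginSalvage and destroying the actor after a short delay.
; BeginSalvage spawns an emitter at the cube, picks a low, average or high value through two separate nested random rolls, and sends it to the player character via AddToSalvageCountMessage.
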(event `/Game/Blueprints/InteractSystem/BPI_Interact.Interact`
  (params (Instigator :type "Actor Object Reference"))
  (`/Engine/EditorBlueprintResources/StandardMacros.DoOnce` false
    (:`Completed`
      (`self.BeginSalvage`)
      (`KismetSystemLibrary.Delay` 0.5)
      (`self.K2_DestroyActor`))))

(fn `BeginSalvage`
  (bind _returnvalue (`KismetMathLibrary.RandomIntegerInRange` 1 10))
  (`GameplayStatics.SpawnEmitterAtLocation` null (`SceneComponent.K2_GetComponentLocation` (`self.Cube`)))
  ;[0.5813 0.9601 1] Roll between 1-10 to decide salvage value
  (if (<= _returnvalue 3)
    ;[1 0.4305 0.2188] Low Salvage Amount
    (bind _output_get (set `self.LowSalvageValue` (`self.LowSalvageValue`)))
    (bind _output_get_2 (set `self.SalvagePileAmount` _output_get))
    (message `/Game/Blueprints/Interfaces/BPI_Salvage.AddToSalvageCount` (`GameplayStatics.GetPlayerCharacter` 0) _output_get_2)
    (elif (<= _returnvalue 9)
      ;[1 0.9352 0.2601] Average Salvage Amount
      (bind _output_get_3 (set `self.AverageSalvageValue` (`self.AverageSalvageValue`)))
      (bind _output_get_4 (set `self.SalvagePileAmount` _output_get_3))
      (message `/Game/Blueprints/Interfaces/BPI_Salvage.AddToSalvageCount` (`GameplayStatics.GetPlayerCharacter` 0) _output_get_4)
      (else
        ;[0.2499 1 0.3458] High Salvage Amount
        (bind _output_get_5 (set `self.HighSalvageValue` (`self.HighSalvageValue`)))
        (bind _output_get_6 (set `self.SalvagePileAmount` _output_get_5))
        (message `/Game/Blueprints/Interfaces/BPI_Salvage.AddToSalvageCount` (`GameplayStatics.GetPlayerCharacter` 0) _output_get_6)))))

(fn `GetInteractHoldTime`
  (returns (HoldTime :type "Float (double-precision)"))
  (return 0.0))

(fn `UserConstructionScript`)