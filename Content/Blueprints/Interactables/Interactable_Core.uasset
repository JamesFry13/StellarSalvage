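; Interactable_Core is a component that detects what the player character faces and sends interact messages to it.
; A forward line trace, run on tick or a looping timer, tracks current and previous hit actors and calls UpdateInteractState, an empty hook here.
; UpdateInteract compares hold duration with the target's hold time before triggering interaction, with a next-tick flag limiting retriggers.
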(event `self.ReceiveBeginPlay`
  (if (`self.UpdateOnTick?`)
    (`self.SetComponentTickEnabled` true)
    (else
      (`KismetSystemLibrary.K2_SetTimer` null "TraceForInteract" (`self.UpdateFrequency`) true))))

(event `self.ReceiveTick`
  (params (DeltaSeconds :type "Float (single-precision)"))
  (`self.TraceForInteract`))

(fn `GetTraceLoc`
  (returns (Start :type "Vector Structure") (End :type "Vector Structure"))
  (bind _returnvalue (`GameplayStatics.GetPlayerCharacter` 0))
  (bind _returnvalue_2 (`Actor.K2_GetActorLocation` _returnvalue))
  (return _returnvalue_2 (+ _returnvalue_2 (* (`Actor.GetActorForwardVector` _returnvalue) 500.0))))

(fn `RetriggerableDelay`
  (if (`self.TriggerDelay`)
    (set `self.TriggerDelay` false)
    (else
      (set `self.TriggerDelay` true)
      (`KismetSystemLibrary.K2_SetTimerForNextTick` null "RetriggerableDelay")
      (message `/Game/Blueprints/Interfaces/BPI_Interact.Interact` (`self.CurrentHitActor`) (`self.GetOwner`))
      (set `self.CurrentHoldDuration` 0.0))))

(fn `StartInteract`
  (`self.RetriggerableDelay`)
  (message `/Game/Blueprints/Interfaces/BPI_Interact.Interact` (`self.CurrentHitActor`) (`self.GetOwner`)))

(fn `TraceForInteract`
  (locals (NewLocalVar :type "Actor Object Reference"))
  (bind (_start _end) (`self.GetTraceLoc`))
  (bind (_outhit _returnvalue) (`KismetSystemLibrary.LineTraceSingle` :`Start` _start :`End` _end :`TraceChannel` "TraceTypeQuery3" :`DrawDebugType` "ForDuration"))
  (if _returnvalue
    (bind (_bblockinghit _binitialoverlap _time _distance _location _impactpoint _normal _impactnormal _physmat _hitactor) (`GameplayStatics.BreakHitResult` _outhit))
    (if (!= _hitactor (`self.CurrentHitActor`))
      (set `self.PrevHitActor` (`self.CurrentHitActor`))
      (set `self.CurrentHitActor` _hitactor)
      (set `self.CanSetPrevious?` true)
      (set `self.CurrentHoldDuration` 0.0)
      (`self.UpdateInteractState` true :!label _label)
      (elif (`self.GetRecheckHit`)
        (`self.DisableHitRecheck`)
        (`self.UpdateInteractState` false)
        (goto _label)))
    (else
      ;[1 1 1] Prevents constant check
      (if (`self.CanSetPrevious?`)
        (`self.DisableHitRecheck`)
        (`/Engine/EditorBlueprintResources/StandardMacros.IsValid` (`self.CurrentHitActor`)
          (:`Is Valid`
            (set `self.PrevHitActor` (`self.CurrentHitActor`)))
          (:`Is Not Valid`
            (set `self.PrevHitActor` null)))
        (set `self.CurrentHitActor` null)
        (set `self.CanSetPrevious?` false)
        (set `self.CurrentHoldDuration` 0.0)
        (`self.UpdateInteractState` false)))))

(fn `UpdateInteract`
  (params (CurrentHoldDuration :type "Float (double-precision)"))
  (set `self.CurrentHoldDuration` CurrentHoldDuration)
  (if (`self.TriggerDelay`)
    _
    (elif (`self.GetCurrentHit`)
      (bind _holdtime (message `/Game/Blueprints/Interfaces/BPI_Interact.GetInteractHoldTime` (`self.CurrentHitActor`)))
      (set `self.InteractHoldTimer` _holdtime)
      (if (>= (`self.InteractHoldTimer`) (`self.CurrentHoldDuration`))
        (`self.StartInteract`)))))

(fn `UpdateInteractState`
  (params (`Hit?` :type Boolean)))